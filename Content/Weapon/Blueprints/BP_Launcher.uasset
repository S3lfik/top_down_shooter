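; BP_Launcher is an automatic rocket launcher weapon that spawns BP_RocketShell actors from its ShootArrow transform.
; PullTrigger, gated by a DoOnce, fires immediately and starts a looping timer at RoundsPerSecond, which ReleaseTrigger clears while resetting the gate.
; Each ConcreteFire call spends ammo, increases spread and increments the shots-made count in the ArenaMode round info, or calls Reload when the ammo is empty.
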(event EventPullTrigger
  (Utilities|FlowControl|DoOnce false
    (:Completed
      (CallFunction|ConcreteFire)
      (bind _returnvalue (Utilities|Time|SetTimerbyFunctionName 0 "ConcreteFire" (/ 1.0 (Variables|Default|GetRoundsPerSecond)) true)))))

(event EventReleaseTrigger
  (Utilities|Time|ClearandInvalidateTimerbyHandle (stale EventPullTrigger _returnvalue))
  (Utilities|FlowControl|DoOnce false) ; enters at Reset
)

(event EventBeginPlay)

(event EventActorBeginOverlap
  (params (OtherActor :type Actor%20Object%20Reference)))

(event EventTick
  (params (DeltaSeconds :type Float%20%28single-precision%29)))

(fn ConstructionScript
  (|CallParentFunction))

(fn ConcreteFire
  (bind _shootarrow (Variables|Default|GetShootArrow))
  (bind _returnvalue (Transformation|GetWorldTransform _shootarrow))
  (if (> (Variables|Default|GetCurrentAmmoCount) 0)
    (Variables|Default|SetCurrentAmmoCount (- (Variables|Default|GetCurrentAmmoCount) 1))
    (Game|SpawnActorfromClass "/Game/Projectiles/BP_RocketShell.BP_RocketShell_C" (Math|Transform|MakeTransform (.location _returnvalue) (.rotation _returnvalue) (.scale _returnvalue)) "Undefined" 0 0)
    (CallFunction|IncreaseSpread 5.0)
    ;[1 1 1] Store shots made count
    (bind _asarena_mode (Utilities|Casting|CastToArenaMode (Game|GetGameMode)))
    (bind _result (Math|Integer|IncrementInt (.shotsweremade (Variables|/Game/Blueprints/GameModes/ArenaMode.ArenaMode_C|GetCurrentRoundInfo _asarena_mode)))
      (:%20%20
        (Utilities|Struct|SetmembersinGameRoundInfo (Variables|/Game/Blueprints/GameModes/ArenaMode.ArenaMode_C|GetCurrentRoundInfo _asarena_mode) _result)))
    (else
      (CallFunction|Reload))))