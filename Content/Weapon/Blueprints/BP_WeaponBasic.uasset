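; Basic weapon actor that spawns plasma projectiles from its ShootArrow and manages clip ammo.
; Fire spends one round per projectile, or calls Reload on an empty clip to refill it instantly.
; Tick decays spread toward its minimum, but IncreaseSpread is never called here and spread does not affect shots.
; PullTrigger, ReleaseTrigger and CalculateShotInfo are empty; the looping-timer automatic-fire logic is disconnected.
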(event Custom|PullTrigger)

(event Custom|ReleaseTrigger)

(event EventBeginPlay
  (Variables|Default|SetCurrentAmmoCount (Variables|Default|GetAmmoClipSize)))

(event EventActorBeginOverlap
  (params (OtherActor :type Actor%20Object%20Reference)))

(event EventTick
  (params (DeltaSeconds :type Float%20%28single-precision%29))
  (Variables|Default|SetDeltaTime DeltaSeconds)
  (if (>= (Variables|Default|GetSpreadCurrent) (Variables|Default|GetSpreadMin))
    (CallFunction|DecreaseSpread (* (Variables|Default|GetDeltaTime) (Variables|Default|GetSpreadDecreaseSpeed)))))

(fn ConstructionScript)

(fn Reload
  (if (< (Variables|Default|GetCurrentAmmoCount) (Variables|Default|GetAmmoClipSize))
    (Variables|Default|SetCurrentAmmoCount (Variables|Default|GetAmmoClipSize))
    (Development|PrintString "Reload")))

(fn Fire
  (bind _shootarrow (Variables|Default|GetShootArrow))
  (bind _returnvalue (Transformation|GetWorldTransform _shootarrow))
  (if (> (Variables|Default|GetCurrentAmmoCount) 0)
    (Variables|Default|SetCurrentAmmoCount (- (Variables|Default|GetCurrentAmmoCount) 1))
    (Game|SpawnActorfromClass "/Game/Projectiles/ProjectilePlazma.ProjectilePlazma_C" (Math|Transform|MakeTransform (.location _returnvalue) (.rotation _returnvalue) (.scale _returnvalue)) "Undefined" 0 0)
    (else
      (CallFunction|Reload))))

(fn DecreaseSpread
  (params (DecreaseAmount :type Float%20%28single-precision%29))
  (if (<= (- (Variables|Default|GetSpreadCurrent) DecreaseAmount) (Variables|Default|GetSpreadMin))
    (Variables|Default|SetSpreadCurrent (Variables|Default|GetSpreadMin))
    (else
      (Variables|Default|SetSpreadCurrent (- (Variables|Default|GetSpreadCurrent) DecreaseAmount)))))

(fn IncreaseSpread
  (params (IncreaseAmount :type Float%20%28single-precision%29))
  (if (>= (+ (Variables|Default|GetSpreadCurrent) IncreaseAmount) (Variables|Default|GetSpreadMax))
    (Variables|Default|SetSpreadCurrent (Variables|Default|GetSpreadMax))
    (else
      (Variables|Default|SetSpreadCurrent (+ (Variables|Default|GetSpreadCurrent) IncreaseAmount)))))

(fn CalculateShotInfo)