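; Weapon actor Blueprint that fires projectiles automatically while its trigger is held.
; PullTrigger passes a DoOnce gate, fires immediately, then starts a looping timer that calls Fire at intervals derived from RoundsPerSecond.
; Fire plays a sound and spawns a ProjectileBP at the ProjectileSpawnPoint transform.
; ReleaseTrigger clears the timer and resets the gate for the next pull.
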(event Custom|ReleaseTrigger
  (Class|KismetSystemLibrary|ClearTimerHandle (stale Custom|PullTrigger _returnvalue))
  (Utilities|FlowControl|DoOnce false) ; enters at Reset
)

(event Custom|Fire
  (bind _projectilespawnpoint (Variables|Default|GetProjectileSpawnPoint))
  (bind _returnvalue (Transformation|GetWorldTransform _projectilespawnpoint))
  (Audio|PlaySoundatLocation 0 (.location _returnvalue))
  (Game|SpawnActorfromClass "/Game/Projectiles/ProjectileBP.ProjectileBP_C" (Math|Transform|MakeTransform (.location _returnvalue) (.rotation _returnvalue) (.scale _returnvalue)) "Undefined" 0 0))

(event Custom|PullTrigger
  (Utilities|FlowControl|DoOnce false
    (:Completed
      (CallFunction|Fire)
      (bind _returnvalue (Utilities|Time|SetTimerbyFunctionName 0 "Fire" (/ 1.0 (Variables|Default|GetRoundsPerSecond)) true)))))

(event EventBeginPlay)

(event EventActorBeginOverlap
  (params (OtherActor :type Actor%20Object%20Reference)))

(event EventTick
  (params (DeltaSeconds :type Float%20%28single-precision%29)))

(fn ConstructionScript)