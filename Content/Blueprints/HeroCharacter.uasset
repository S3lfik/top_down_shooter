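; Player hero Character for an arena shooter with world-axis movement and mouse aiming.
; BeginPlay attaches a spawned weapon to the gun socket, passes the spawn transform to ArenaMode and creates the HUD.
; Mouse movement smoothly turns only the mesh toward the cursor, using the character's screen-projected position; Fire drives the weapon trigger.
; On death, AffectHealth disables input, then after a delay requests respawn, destroys hero and weapon, and deducts a life.
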(event EventAffectHealth
  (params (Delta :type Float%20%28single-precision%29))
  (bind _game_mode (Variables|Default|GetGame%20mode))
  ;[1 1 1] Damage process
  (Class|BaseCharacter|CalculateHealth Delta)
  (if (Variables|Default|Get_isDead)
    (Input|DisableInput 0)
    (Utilities|FlowControl|Delay 2.0)
    (Default|RespawnPlayer _game_mode)
    (Actor|DestroyActor (Variables|Default|GetWeapon))
    (Default|ChangeLives _game_mode -1)))

(event EventBeginPlay
  (bind _mesh (Variables|Character|GetMesh))
  (Utilities|FlowControl|Sequence
    (:then_0
      ;[1 1 1] Setup weapon
      (bind _returnvalue (Game|SpawnActorfromClass "/Game/Blueprints/Weapon.Weapon_C" (Transformation|GetWorldTransform _mesh) "Undefined" 0 0))
      (bind _output_get (Variables|Default|SetWeapon _returnvalue))
      (Class|Actor|AttachRootComponentto _output_get _mesh "Gun_Socket" "SnapToTarget" true))
    (:then_1
      ;[1 1 1] Send Player Transform to Mode
      (bind _asarena_mode (Utilities|Casting|CastToArenaMode (Game|GetGameMode)))
      (bind _output_get_2 (Variables|Default|SetGame%20mode _asarena_mode))
      (Variables|/Game/Blueprints/GameModes/ArenaMode.ArenaMode_C|SetPlayerSpawnTransform _output_get_2 (Transformation|GetActorTransform)))
    (:then_2
      ;[1 1 1] Set HUD
      (bind _returnvalue_2 (UserInterface|CreateWidget "/Game/Blueprints/ArenaHUD.ArenaHUD_C"))
      (UserInterface|Viewport|AddtoViewport _returnvalue_2 0))))

(event EventActorBeginOverlap
  (params (OtherActor :type Actor%20Object%20Reference)))

(event EventTick
  (params (DeltaSeconds :type Float%20%28single-precision%29))
  ;[1 1 1] Tick Setup
  (Variables|Default|SetTickTime DeltaSeconds))

(event Input|ActionEvents|InputActionFire
  (params (Key :type Key%20Structure :default "AnyKey"))
  (bind _weapon (Variables|Default|GetWeapon))
  ;[1 1 1] Firing
  (:Pressed
    (Default|PullTrigger _weapon))
  (:Released
    (Default|ReleaseTrigger _weapon)))

(event Input|AxisEvents|InputAxisMoveUp
  (params (AxisValue :type Float%20%28single-precision%29))
  ;[1 1 1] Movement
  (Pawn|Input|AddMovementInput "1.000000, 0, 0" AxisValue false))

(event Input|AxisEvents|InputAxisMoveRight
  (params (AxisValue :type Float%20%28single-precision%29))
  ;[1 1 1] Movement
  (Pawn|Input|AddMovementInput "0,1.000000, 0" AxisValue false))

(event Input|MouseEvents|MouseX
  (params (AxisValue :type Float%20%28single-precision%29))
  (bind _returnvalue (Game|GetPlayerController 0))
  (bind _returnvalue_2 (Game|GetPlayerCharacter 0))
  (bind _mesh (Variables|Character|GetMesh))
  (bind _returnvalue_3 (Transformation|GetActorLocation _returnvalue_2))
  (bind (_locationx _locationy _returnvalue_4) (Game|Player|GetMousePosition _returnvalue))
  (bind _relativerotation (Variables|/Script/Engine.SceneComponent|GetRelativeRotation _mesh))
  (bind _screenlocation (Class|PlayerController|ProjectWorldLocationtoScreen _returnvalue _returnvalue_3))
  ;[1 1 1] Rotation
  (if _returnvalue_4 ; If no mouse, do nothing
    (Transformation|SetRelativeRotation _mesh (Math|Rotator|Lerp(Rotator) _relativerotation (Math|Rotator|MakeRotator 0.0 0.0 (.yaw (Math|Interpolation|RInterpTo _relativerotation (Math|Rotator|MakeRotfromX (Class|KismetMathLibrary|GetDirectionVector (Math|Vector|MakeVector (.x _screenlocation) (.y _screenlocation) 0.0) (Math|Vector|MakeVector _locationx _locationy 0.0))) (Variables|Default|GetTickTime) 1e+01))) 1e+01 true) false false)))

(event Input|MouseEvents|MouseY
  (params (AxisValue :type Float%20%28single-precision%29))
  (bind _returnvalue (Game|GetPlayerController 0))
  (bind _returnvalue_2 (Game|GetPlayerCharacter 0))
  (bind _mesh (Variables|Character|GetMesh))
  (bind _returnvalue_3 (Transformation|GetActorLocation _returnvalue_2))
  (bind (_locationx _locationy _returnvalue_4) (Game|Player|GetMousePosition _returnvalue))
  (bind _relativerotation (Variables|/Script/Engine.SceneComponent|GetRelativeRotation _mesh))
  (bind _screenlocation (Class|PlayerController|ProjectWorldLocationtoScreen _returnvalue _returnvalue_3))
  ;[1 1 1] Rotation
  (if _returnvalue_4 ; If no mouse, do nothing
    (Transformation|SetRelativeRotation _mesh (Math|Rotator|Lerp(Rotator) _relativerotation (Math|Rotator|MakeRotator 0.0 0.0 (.yaw (Math|Interpolation|RInterpTo _relativerotation (Math|Rotator|MakeRotfromX (Class|KismetMathLibrary|GetDirectionVector (Math|Vector|MakeVector (.x _screenlocation) (.y _screenlocation) 0.0) (Math|Vector|MakeVector _locationx _locationy 0.0))) (Variables|Default|GetTickTime) 1e+01))) 1e+01 true) false false)))

(fn ConstructionScript)