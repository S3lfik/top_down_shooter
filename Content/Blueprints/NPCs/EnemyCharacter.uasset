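; Enemy NPC character that melee-attacks the hero and, on death, adds score to ArenaMode and drops a health pickup.
; Construction tints the body through a dynamic material and snaps colliders to both hands.
; Attack and StopAttack toggle those colliders, and overlapping the hero deals damage once, as the repeating damage timer is unconnected.
; Death stops attacks, then progressively ignores collision channels before destroying the actor.
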(event Custom|PlayDead
  ;[1 1 1] Set deadness of character
  (CallFunction|StopAttack))

(event Custom|Attack
  ;[1 1 1] Switching Damaging collisions
  (Variables|Default|SetisAttacking (not (Variables|Default|Get_isDead)))
  (Collision|SetCollisionEnabled (Variables|Default|GetRightHandCollider) "QueryOnly"))

(event Custom|StopAttack
  ;[1 1 1] Switching Damaging collisions
  (Variables|Default|SetisAttacking false)
  (Collision|SetCollisionEnabled (Variables|Default|GetRightHandCollider) "NoCollision"))

(event Custom|DamageTheHero
  (Default|AffectHealth (Variables|Default|GetHero) (Variables|Default|GetDamage)))

(event Custom|CheckDrop
  (bind _mesh (Variables|Character|GetMesh))
  (bind _returnvalue (Transformation|GetWorldTransform _mesh))
  ;[1 1 1] Check pickup drop
  (Game|SpawnActorfromClass "/Game/Blueprints/Pickups/HealthPickup_BP.HealthPickup_BP_C" (Math|Transform|MakeTransform (Math|Vector|MakeVector (.x (.location _returnvalue)) (.y (.location _returnvalue)) 9e+01) (Math|Conversions|RotationFromXVector "0.000000, 0, 0") (.scale _returnvalue)) "Undefined" 0 0))

(event Collision|EventActorEndOverlap
  (params (OtherActor :type Actor%20Object%20Reference))
  (if (== OtherActor (Variables|Default|GetHero))
    (Class|KismetSystemLibrary|ClearTimerHandle (stale _returnvalue))))

(event EventAffectHealth
  (params (Delta :type Float%20%28single-precision%29))
  (bind _capsulecomponent (Variables|Default|GetCapsuleComponent))
  (Class|BaseCharacter|CalculateHealth Delta)
  (if (Variables|Default|Get_isDead)
    (CallFunction|PlayDead)
    (bind _asarena_mode (Utilities|Casting|CastToArenaMode (Game|GetGameMode)))
    (Default|IncreaseScore _asarena_mode (Variables|Default|GetScore))
    (Collision|SetCollisionResponsetoChannel _capsulecomponent "ECC_WorldDynamic" "ECR_Ignore")
    (Collision|SetCollisionResponsetoChannel _capsulecomponent "ECC_Pawn" "ECR_Ignore")
    (CallFunction|CheckDrop)
    (Utilities|FlowControl|Delay 2.5)
    (Collision|SetCollisionResponsetoChannel _capsulecomponent "ECC_WorldStatic" "ECR_Ignore")
    (Utilities|FlowControl|Delay 1.0)
    (AI|GetAIController 0)
    (Class|Pawn|DetachfromControllerPendingDestroy)
    (Actor|DestroyActor)))

(event EventBeginPlay
  (Collision|SetCollisionEnabled (Variables|Default|GetRightHandCollider) "NoCollision"))

(event EventActorBeginOverlap
  (params (OtherActor :type Actor%20Object%20Reference))
  (bind _ashero_character (Utilities|Casting|CastToHeroCharacter OtherActor))
  (Variables|Default|SetHero _ashero_character)
  (CallFunction|DamagetheHero))

(event EventTick
  (params (DeltaSeconds :type Float%20%28single-precision%29)))

(fn ConstructionScript
  (bind _mesh (Variables|Character|GetMesh))
  (bind _returnvalue (Rendering|Material|CreateDynamicMaterialInstance _mesh 0 "/Game/AnimationAssets/UE4_Mannequin/Materials/M_UE4Man_Body.M_UE4Man_Body" :!class /Script/Engine.PrimitiveComponent))
  (bind _output_get (Variables|Default|SetDynaMat _returnvalue))
  (Rendering|Material|SetVectorParameterValue _output_get "BodyColor" (Variables|Default|GetEnemyColor) :!class /Script/Engine.MaterialInstanceDynamic)
  (Class|SceneComponent|Attachto (Variables|Default|GetLeftHandCollision) _mesh "hand_l" "SnapToTarget" true)
  (Class|SceneComponent|Attachto (Variables|Default|GetRightHandCollider) _mesh "hand_r" "SnapToTarget" true))