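; EnemyAIController is the AI controller that makes an enemy chase and attack the player character.
; A looping half-second timer runs TrackPlayer, which moves the pawn toward the player within AIAttackRange.
; Reaching the player starts the enemy's attack if not already attacking, and a failed move stops it.
; A dead player halts movement and attacking, while a dead enemy only halts movement.
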(event Custom|TrackPlayer
  (bind _returnvalue (Pawn|GetControlledPawn))
  (if (Variables|/Script/TopDownShooter.BaseCharacter|Get_isDead (Variables|Default|GetTarget))
    ;[1 1 1] If target is dead (and is only)
    (AI|Navigation|StopMovement)
    ;;[1 1 1] !stopAttack
    (bind _asenemy_character (Utilities|Casting|CastToEnemyCharacter (Pawn|GetControlledPawn)))
    (Default|StopAttack _asenemy_character)
    (else
      (bind _asenemy_character_2 (Utilities|Casting|CastToEnemyCharacter _returnvalue))
      (bind _output_get (Variables|Default|SetControlledCharacter _asenemy_character_2))
      (if (Variables|/Script/TopDownShooter.BaseCharacter|Get_isDead _output_get)
        (AI|Navigation|StopMovement)
        (else
          (AI|AIMoveTo _returnvalue "0, 0, 0" (Game|GetPlayerCharacter 0) (Variables|Default|GetAIAttackRange) true
            (:OnSuccess
              (if (not (Variables|/Game/Blueprints/NPCs/EnemyCharacter.EnemyCharacter_C|GetisAttacking (Variables|Default|GetControlledCharacter)))
                ;[1 1 1] !attack
                (Default|Attack (Variables|Default|GetControlledCharacter))))
            (:OnFail
              (if (Variables|/Game/Blueprints/NPCs/EnemyCharacter.EnemyCharacter_C|GetisAttacking (Variables|Default|GetControlledCharacter))
                (Default|StopAttack (Variables|Default|GetControlledCharacter))))))))))

(event EventBeginPlay
  (bind _asbase_character (Utilities|Casting|CastToBaseCharacter (Game|GetPlayerCharacter 0))
    (:then
      (Variables|Default|SetTarget _asbase_character))
    (:CastFailed
      _))
  (Utilities|Time|SetTimerbyFunctionName 0 "TrackPlayer" 0.5 true))

(event EventTick
  (params (DeltaSeconds :type Float%20%28single-precision%29)))

(fn ConstructionScript)