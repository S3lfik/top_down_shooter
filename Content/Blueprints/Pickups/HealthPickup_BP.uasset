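; Health pickup actor that heals the hero character on overlap and then destroys itself.
; A cast to HeroCharacter filters the overlap, but the heal targets the player 0 character rather than the overlapping actor.
; It reduces HealPower to the missing health so the total stays within a hard-coded maximum of 100, then passes it to AffectHealth.
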(event Custom|applyPickup
  ;[1 1 1] Apply heal effect
  (bind _ashero_character (Utilities|Casting|CastToHeroCharacter (Game|GetPlayerCharacter 0)))
  (if (<= (+ (Variables|Default|GetHealPower) (Variables|/Script/TopDownShooter.BaseCharacter|Get_health _ashero_character)) 1e+02) ; If Heal power is lower than the lack of HP
    _
    (else
      (Variables|Default|SetHealPower (- 1e+02 (Variables|/Script/TopDownShooter.BaseCharacter|Get_health _ashero_character)))))
  (Default|AffectHealth _ashero_character (Variables|Default|GetHealPower)))

(event EventBeginPlay)

(event EventActorBeginOverlap
  (params (OtherActor :type Actor%20Object%20Reference))
  ;[1 1 1] Overlap works only for hero character
  (Utilities|Casting|CastToHeroCharacter OtherActor)
  (CallFunction|ApplyPickup)
  (Actor|DestroyActor))

(event EventTick
  (params (DeltaSeconds :type Float%20%28single-precision%29)))

(fn ConstructionScript)