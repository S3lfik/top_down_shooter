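; Enemy spawner actor that adds red or blue boxer AI enemies at random points inside its SpawnVolume.
; SpawnEnemy counts all BaseEnemy actors in the world and spawns only while that count is below EnemyLimit.
; Each call spawns one BoxerRed or BoxerBlue with equal odds.
; Nothing in this graph calls SpawnEnemy, as BeginPlay, overlap and Tick are unused.
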(event Custom|SpawnEnemy
  (bind _spawnvolume (Variables|Default|GetSpawnVolume))
  (bind _returnvalue (Components|Box|GetScaledBoxExtent _spawnvolume))
  (bind _returnvalue_2 (Transformation|GetWorldLocation _spawnvolume))
  (bind _returnvalue_3 (Math|Random|RandomPointinBoundingBox _returnvalue_2 _returnvalue))
  ;[1 1 1] EnemySpawn
  (bind _outactors (Actor|GetAllActorsOfClass "/Game/Blueprints/NPCs/BaseEnemy.BaseEnemy_C"))
  (if (< (Utilities|Array|Length _outactors) (Variables|Default|GetEnemyLimit))
    (if (> (Math|Random|RandomIntegerinRange 0 1) 0)
      (AI|SpawnAIFromClass "/Game/Blueprints/NPCs/Boxer/BoxerRed.BoxerRed_C" 0 _returnvalue_3 "0, 0, 0" false)
      (else
        (AI|SpawnAIFromClass "/Game/Blueprints/NPCs/Boxer/BoxerBlue.BoxerBlue_C" 0 _returnvalue_3 "0, 0, 0" false)))))

(event EventBeginPlay)

(event EventActorBeginOverlap
  (params (OtherActor :type Actor%20Object%20Reference)))

(event EventTick
  (params (DeltaSeconds :type Float%20%28single-precision%29)))

(fn ConstructionScript)