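; Main menu game mode that shows a splash screen on BeginPlay, then adds the main menu widget after a short timer.
; Show events for the main, settings, credits and single-player menus lazily create and cache their widgets, add them to the viewport and set focused UI-only input with a cursor.
; The timed StartMenu creates its main menu widget without caching it, and nothing here removes the splash or other widgets.
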(event Custom|StartMenu
  (bind _returnvalue (UserInterface|CreateWidget "/Game/UI/MainMenu/MainMenuWidget.MainMenuWidget_C"))
  (UserInterface|Viewport|AddtoViewport _returnvalue 0))

(event Custom|ShowMainMenu
  (bind _returnvalue (Game|GetPlayerController 0))
  (if (Utilities|IsValid (Variables|Default|GetMainMenuWidget))
    _
    (else
      (bind _returnvalue_2 (UserInterface|CreateWidget "/Game/UI/MainMenu/MainMenuWidget.MainMenuWidget_C"))
      (Variables|Default|SetMainMenuWidget _returnvalue_2)))
  (UserInterface|Viewport|AddtoViewport (Variables|Default|GetMainMenuWidget) 0)
  (Input|SetInputModeUIOnly _returnvalue (Variables|Default|GetMainMenuWidget) "DoNotLock")
  (Variables|/Script/Engine.PlayerController|SetbShowMouseCursor _returnvalue true))

(event Custom|ShowCreditsMenu
  (bind _returnvalue (Game|GetPlayerController 0))
  (if (Utilities|IsValid (Variables|Default|GetCreditsMenuWidget))
    _
    (else
      (bind _returnvalue_2 (UserInterface|CreateWidget "/Game/UI/MainMenu/CreditsMenuWidget.CreditsMenuWidget_C"))
      (Variables|Default|SetCreditsMenuWidget _returnvalue_2)))
  (UserInterface|Viewport|AddtoViewport (Variables|Default|GetCreditsMenuWidget) 0)
  (Input|SetInputModeUIOnly _returnvalue (Variables|Default|GetCreditsMenuWidget) "DoNotLock")
  (Variables|/Script/Engine.PlayerController|SetbShowMouseCursor _returnvalue true))

(event Custom|ShowSinglePlayerMenu
  (bind _returnvalue (Game|GetPlayerController 0))
  (if (Utilities|IsValid (Variables|Default|GetSinglePlayerMenuWidget))
    _
    (else
      (bind _returnvalue_2 (UserInterface|CreateWidget "/Game/UI/MainMenu/SinglePlayerMenuWidget.SinglePlayerMenuWidget_C"))
      (Variables|Default|SetSinglePlayerMenuWidget _returnvalue_2)))
  (UserInterface|Viewport|AddtoViewport (Variables|Default|GetSinglePlayerMenuWidget) 0)
  (Input|SetInputModeUIOnly _returnvalue (Variables|Default|GetSinglePlayerMenuWidget) "DoNotLock")
  (Variables|/Script/Engine.PlayerController|SetbShowMouseCursor _returnvalue true))

(event Custom|ShowSettingsMenu
  (bind _returnvalue (Game|GetPlayerController 0))
  (if (Utilities|IsValid (Variables|Default|GetSettingsMenuWidget))
    _
    (else
      (bind _returnvalue_2 (UserInterface|CreateWidget "/Game/UI/MainMenu/SettingsMenuWidget.SettingsMenuWidget_C"))
      (Variables|Default|SetSettingsMenuWidget _returnvalue_2)))
  (UserInterface|Viewport|AddtoViewport (Variables|Default|GetSettingsMenuWidget) 0)
  (Input|SetInputModeUIOnly _returnvalue (Variables|Default|GetSettingsMenuWidget) "DoNotLock")
  (Variables|/Script/Engine.PlayerController|SetbShowMouseCursor _returnvalue true))

(event EventBeginPlay
  (bind _returnvalue (Game|GetPlayerController 0))
  (bind _returnvalue_2 (UserInterface|CreateWidget "/Game/UI/MainMenu/SplashWidget.SplashWidget_C"))
  (UserInterface|Viewport|AddtoViewport _returnvalue_2 0)
  (Input|SetInputModeUIOnly _returnvalue 0 "LockOnCapture")
  (Variables|/Script/Engine.PlayerController|SetbShowMouseCursor _returnvalue true)
  (Utilities|Time|SetTimerbyEvent (delegate Custom|StartMenu) 2.0)
  (Development|PrintString "GameMode::Loaded"))

(fn ConstructionScript)