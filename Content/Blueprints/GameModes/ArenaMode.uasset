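; ArenaMode is the game mode for an arena game, managing enemy spawning, score, lives and game over.
; On begin play it sets a looping timer on the first EnemySpawner found, calling SpawnEnemy at SpawnsPerSecond.
; RespawnPlayer destroys all live enemies, then spawns and possesses a new HeroCharacter at the stored spawn transform.
; Events adjust score and lives; depleted lives trigger GameOver, which resets the level and opens the game-over map.
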(event Custom|RespawnPlayer
  ;[1 1 1] RespawnPlayer
  (bind _outactors (Actor|GetAllActorsOfClass "/Game/Characters/NPCs/BaseEnemy.BaseEnemy_C")) ; Get all enemy characters to clear the arena
  (for _array_element _outactors
    (Actor|DestroyActor _array_element) ; Destroy all enemies that are currently alive
  )
  (bind _returnvalue (Game|SpawnActorfromClass "/Game/Characters/HeroCharacter.HeroCharacter_C" (Variables|Default|GetPlayerSpawnTransform) "AdjustIfPossibleButAlwaysSpawn" 0 0))
  (Pawn|Possess (Game|GetPlayerController 0) _returnvalue))

(event Custom|IncreaseScore
  (params (DeltaScore :type Integer))
  (Variables|Default|SetScore (+ DeltaScore (Variables|Default|GetScore))))

(event Custom|ChangeLives
  (params (Delta :type Integer))
  (bind _output_get (Variables|Default|SetLives (+ Delta (Variables|Default|GetLives))))
  (if (<= _output_get 0)
    (CallFunction|GameOver)))

(event Custom|GameOver
  (Variables|Default|SetisGameOver true)
  (Class|GameModeBase|ResetLevel)
  (Game|OpenLevel(byName) "GameOverMap"))

(event EventBeginPlay
  (Utilities|FlowControl|Sequence
    (:then_0
      ;[1 1 1] SpawnEnemies
      (bind _outactors (Actor|GetAllActorsOfClass "/Game/Blueprints/EnemySpawner.EnemySpawner_C"))
      (bind _output_get (Variables|Default|SetSpawner (Utilities|Array|Get(acopy) _outactors)))
      (Utilities|Time|SetTimerbyFunctionName _output_get "SpawnEnemy" (/ 1.0 (Variables|Default|GetSpawnsPerSecond)) true))))

(event EventTick
  (params (DeltaSeconds :type Float%20%28single-precision%29)))

(fn ConstructionScript)