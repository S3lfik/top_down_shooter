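; ProjectileBP is a projectile actor, apparently a laser given its LeserMesh, that damages hostile actors on overlap.
; It filters overlaps through the IDamageable interface, then sends Damage via AffectHealthMessage to targets without the "Friendly" tag, with sound and particle effects spawned at the mesh.
; It destroys itself on any damageable overlap, friendly or not, and ignores all other actors.
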(event EventBeginPlay)

(event EventActorBeginOverlap
  (params (OtherActor :type Actor%20Object%20Reference))
  (bind _lesermesh (Variables|Default|GetLeserMesh))
  (bind _returnvalue (Transformation|GetWorldTransform _lesermesh))
  (if (Utilities|DoesObjectImplementInterface OtherActor "/Game/Blueprints/iDamageable.iDamageable_C")
    (if (not (Actor|ActorHasTag OtherActor "Friendly"))
      (Class|IDamageable|AffectHealth(Message) OtherActor (Variables|Default|GetDamage))
      (Audio|PlaySoundatLocation 0 (.location _returnvalue))
      (Effects|SpawnEmitteratLocation 0 (.location _returnvalue) (.rotation _returnvalue)))
    (Actor|DestroyActor)))

(event EventTick
  (params (DeltaSeconds :type Float%20%28single-precision%29)))

(fn ConstructionScript)