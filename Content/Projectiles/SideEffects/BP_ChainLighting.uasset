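; BP_ChainLighting is a chain lightning actor that jumps between BaseEnemy actors, each instance handling one link.
; Activate damages the first enemy within JumpMaxDistance of PreviousTarget that is absent from the Sender hit list.
; It draws a beam between their hit sockets, then spawns and activates the next link with modified damage and remaining jumps.
; Each link self-destructs after a short delay or when no target or jumps remain.
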(event Custom|Activate
  (bind _sender (Variables|Default|GetSender))
  (bind _returnvalue (Utilities|Array|Length _sender))
  (if (> (Variables|Default|GetJumps) 0)
    (Variables|Default|SetJumps (- (Variables|Default|GetJumps) 1))
    (Utilities|FlowControl|Sequence
      (:then_0
        (Utilities|IsValid (Variables|Default|GetPreviousTarget)
          (:Is%20Valid
            ;[1 1 1] If prev. target is valid, push it into array
            (Utilities|Array|AddUnique (Variables|Default|GetSender) (Variables|Default|GetPreviousTarget)))
          (:Is%20Not%20Valid
            ;[1 1 1] If not, take the last element of non-empty array
            (if (> _returnvalue 0)
              (Variables|Default|SetPreviousTarget (Utilities|Array|Get(acopy) (Variables|Default|GetSender) (- _returnvalue 1)))
              (else
                (Development|PrintString "oops"))))))
      (:then_1
        (bind _result (CallFunction|InitTarget))
        (if _result
          (Development|PrintString "Valid")
          (Default|AffectHealth (Variables|Default|GetTarget) (Variables|Default|GetDamage))
          (bind _newparam (CallFunction|SpawnEmitter))
          (Variables|Default|SetLightingEffectComponent _newparam)
          (CallFunction|CreateNextLink)
          ;[1 1 1] Destroy
          (Utilities|FlowControl|Delay 0.15)
          (Components|DestroyComponent (Variables|Default|GetStaticMesh))
          (Components|DestroyComponent (Variables|Default|GetLightingEffectComponent))
          (Actor|DestroyActor)
          (else
            (Development|PrintString "Invalid")
            (Components|DestroyComponent (Variables|Default|GetStaticMesh))
            (Actor|DestroyActor)))))
    (else
      (Actor|DestroyActor))))

(event EventBeginPlay)

(event Collision|EventActorBeginOverlap
  (params (OtherActor :type Actor%20Object%20Reference)))

(event EventTick
  (params (DeltaSeconds :type Float%20%28single-precision%29)))

(fn ConstructionScript)

(fn InitTarget
  ;[1 1 1] If we have enemies
  (bind _outactors (Actor|GetAllActorsOfClass "/Game/Characters/NPCs/BaseEnemy.BaseEnemy_C"))
  (if (> (Utilities|Array|Length _outactors) 0)
    (bind _array_element (Utilities|Array|ForEachLoopwithBreak _outactors :!label _label)
      (:LoopBody
        (LocalVariables|SetEnemiesIterator _array_element)
        (if (not (Utilities|Array|ContainsItem (Variables|Default|GetSender) (LocalVariables|GetEnemiesIterator)))
          (if (<= (Math|Float|Absolute(Float) (Math|Vector|VectorLength (- (Transformation|GetWorldLocation (Variables|/Script/Engine.Character|GetMesh (Variables|Default|GetPreviousTarget))) (Transformation|GetWorldLocation (Variables|/Script/Engine.Character|GetMesh (LocalVariables|GetEnemiesIterator)))))) (Variables|Default|GetJumpMaxDistance))
            (Variables|Default|SetTarget (LocalVariables|GetEnemiesIterator))
            (goto _label Break))))
      (:Completed
        (Utilities|IsValid (Variables|Default|GetTarget)
          (:Is%20Valid
            (Utilities|Array|Add (Variables|Default|GetSender) (Variables|Default|GetTarget))
            (return true))
          (:Is%20Not%20Valid
            (return false)))))
    (else
      (return false))))

(fn SpawnEmitter
  (bind _returnvalue (Effects|SpawnEmitteratLocation "/Game/Projectiles/Particles/P_Lighting.P_Lighting" (Transformation|GetSocketLocation (Variables|/Script/Engine.Character|GetMesh (Variables|Default|GetPreviousTarget)) "hit_socket")))
  (bind _output_get (LocalVariables|SetLighting _returnvalue))
  (Class|ParticleSystemComponent|SetBeamTargetPoint _output_get 0 (Transformation|GetSocketLocation (Variables|/Script/Engine.Character|GetMesh (Variables|Default|GetTarget)) "hit_socket"))
  (return (LocalVariables|GetLighting)))

(fn CreateNextLink
  (bind _returnvalue (Game|SpawnActorfromClass "BP_ChainLighting_C" (Transformation|GetWorldTransform (Variables|Default|GetStaticMesh)) "Undefined" 0 0))
  (Variables|BP_ChainLighting_C|SetDamage _returnvalue (* (Variables|Default|GetDamage) (Variables|Default|GetDamageStepModifier)))
  (Variables|BP_ChainLighting_C|SetJumpMaxDistance _returnvalue (Variables|Default|GetJumpMaxDistance))
  (Variables|BP_ChainLighting_C|SetJumps _returnvalue (Variables|Default|GetJumps))
  (Variables|BP_ChainLighting_C|SetPreviousTarget _returnvalue (Variables|Default|GetTarget))
  (Variables|BP_ChainLighting_C|SetSender _returnvalue (Variables|Default|GetSender))
  (CallFunction|Activate _returnvalue))