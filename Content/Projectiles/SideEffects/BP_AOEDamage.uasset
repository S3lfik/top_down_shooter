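; BP_AOEDamage is a projectile side effect that creates an explosion dealing area damage when activated, then destroys itself after a short delay.
; Activate resizes a debug sphere, spawns a radius-scaled explosion particle, and plays a camera shake, plus a sound at world origin.
; It finds damageable actors by interface and applies flat damage to each BaseCharacter whose mesh is within EffectRadius, using distance checks rather than overlaps.
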(event Custom|Activate
  (bind _sphere (Variables|Default|GetSphere))
  (bind _returnvalue (Transformation|GetWorldLocation _sphere))
  (Utilities|FlowControl|Sequence
    (:then_0
      ;[1 1 1] Draw debug sphere
      (Components|Sphere|SetSphereRadius (Variables|Default|GetSphere) (* (Variables|Default|GetEffectRadius) 1e+01) true))
    (:then_1
      (bind _returnvalue_2 (Effects|SpawnEmitteratLocation "/Game/StarterContent/Particles/P_Explosion.P_Explosion" _returnvalue))
      (bind _output_get (Variables|Default|SetParticleSystemScaleFactor (/ (Variables|Default|GetEffectRadius) 125.0)))
      (Transformation|SetRelativeScale3D _returnvalue_2 (Math|Vector|MakeVector _output_get _output_get _output_get))
      (Camera|PlayWorldCameraShake "/Game/Projectiles/RocketLauncherCameraShake.RocketLauncherCameraShake_C" _returnvalue 0.0 1.2e+03)
      (Audio|PlaySoundatLocation "/Game/StarterContent/Audio/Explosion_Cue.Explosion_Cue" "0, 0, 0"))
    (:then_2
      (bind _outactors (Actor|GetAllActorswithInterface "/Game/Blueprints/iDamageable.iDamageable_C"))
      (for _array_element _outactors
        (bind _asbase_character (Utilities|Casting|CastToBaseCharacter _array_element))
        (if (< (Math|Vector|VectorLength (- (Transformation|GetWorldLocation (Variables|Default|GetDefaultSceneRoot)) (Transformation|GetWorldLocation (Variables|/Script/Engine.Character|GetMesh _asbase_character)))) (Variables|Default|GetEffectRadius))
          (Class|IDamageable|AffectHealth(Message) _asbase_character (Variables|Default|GetDamage))))
      (Utilities|FlowControl|Delay 1.0)
      (Actor|DestroyActor))))

(event EventBeginPlay)

(event Collision|EventActorBeginOverlap
  (params (OtherActor :type Actor%20Object%20Reference)))

(event EventTick
  (params (DeltaSeconds :type Float%20%28single-precision%29)))

(fn ConstructionScript)