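; BP_RocketShell is a rocket projectile that deals direct hit damage and an area explosion.
; On actor overlap, CheckEnemyHit filters the other actor, and a valid hit receives Damage through AffectHealthMessage.
; It then spawns a BP_AOEDamage at the shell mesh's transform, passes it the explosion radius and damage, activates it and destroys itself.
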(event EventBeginPlay)

(event Collision|EventActorBeginOverlap
  (params (OtherActor :type Actor%20Object%20Reference))
  (bind _ishit (CallFunction|CheckEnemyHit OtherActor))
  (if _ishit
    (Class|IDamageable|AffectHealth(Message) OtherActor (Variables|Default|GetDamage))
    (bind _returnvalue (Game|SpawnActorfromClass "/Game/Projectiles/SideEffects/BP_AOEDamage.BP_AOEDamage_C" (Transformation|GetWorldTransform (Variables|Default|GetShellMesh)) "Undefined" 0 0))
    (Variables|/Game/Projectiles/SideEffects/BP_AOEDamage.BP_AOEDamage_C|SetEffectRadius _returnvalue (Variables|Default|GetExplsionRadius))
    (Variables|/Game/Projectiles/SideEffects/BP_AOEDamage.BP_AOEDamage_C|SetDamage _returnvalue (Variables|Default|GetExplosionDamage))
    (Default|Activate _returnvalue)
    (Actor|DestroyActor)))

(event EventTick
  (params (DeltaSeconds :type Float%20%28single-precision%29)))

(fn ConstructionScript
  (|CallParentFunction))